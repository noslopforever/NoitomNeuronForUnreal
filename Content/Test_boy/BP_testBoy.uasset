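; BP_testBoy is a test actor that is driven by Neuron motion capture data received over UDP.
; On BeginPlay it connects on port 7001 as actor 0 and hands the resulting proxy to the mesh's NeuronAnimInstance.
; Each tick it transforms the captured hip movement to world space and applies the change from the cached previous position as an unswept actor offset, so the actor follows the performer.
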(event `self.ReceiveBeginPlay`
  ;[1 1 1] Initialize Neuron Actor Proxy and apply it to animation if needed.
  (bind _asneuron_anim_instance (cast `NeuronAnimInstance` (`SkeletalMeshComponent.GetAnimInstance` (`self.Mesh`))))
  (bind _returnvalue (`NeuronActorProxy.ConnectUDP` 7001))
  (`NeuronAnimInstance.SetNeuronProxy` _asneuron_anim_instance _returnvalue)
  (bind _output_get (set `self.NeuronActorProxy` _returnvalue))
  ;;[1 1 1] Get world space translation
  (set `self.AnimationTranslation` (`KismetMathLibrary.TransformLocation` (`SceneComponent.K2_GetComponentToWorld` (`self.Mesh`)) (`NeuronBPLibrary.GetNeuronActorHipMoveCS` _output_get))))

(event `self.ReceiveActorBeginOverlap`
  (params (OtherActor :type "Actor Object Reference")))

(event `self.ReceiveTick`
  (params (DeltaSeconds :type "Float (single-precision)"))
  (bind _neuronactorproxy (`self.NeuronActorProxy`))
  (bind _returnvalue (`KismetMathLibrary.TransformLocation` (`SceneComponent.K2_GetComponentToWorld` (`self.Mesh`)) (`NeuronBPLibrary.GetNeuronActorHipMoveCS` _neuronactorproxy)))
  ;[1 1 1] Apply Neuron movement
  (`|ExecutionSequence`
    (:`then_0`
      (`/Engine/EditorBlueprintResources/StandardMacros.IsValid` _neuronactorproxy
        (:`Is Valid`
          (`self.K2_AddActorWorldOffset` (- _returnvalue (`self.AnimationTranslation`))))))
    (:`then_1`
      (set `self.AnimationTranslation` _returnvalue) ; Cache this frame translation
    )))

(fn `UserConstructionScript`)